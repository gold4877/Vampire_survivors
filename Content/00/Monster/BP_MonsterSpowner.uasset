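; Monster spawner that attempts every second to place a random monster on a circle around its owner.
; The circle's radius is Radius times 2π, and a spot qualifies when a WorldDynamic line trace hits.
; That trace's end multiplies the location by a downward vector instead of adding an offset.
; A random DT_monster row supplies the class, spawned with BT_Monster facing the owner and initialized through InitMonsterInfo.
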(event EventBeginPlay
  (Utilities|Time|SetTimerbyFunctionName 0 "DoSpawn" 1.0 true))

(event EventTick
  (params (DeltaSeconds :type Float%20%28single-precision%29)))

(fn DoSpawn
  (bind _returnvalue (Components|GetOwner))
  (bind _radius (Variables|Default|GetRadius))
  (bind _returnvalue_2 (Transformation|GetActorLocation _returnvalue))
  (bind _returnvalue_3 (* _radius 2.0 3.141592))
  (bind _output_get (LocalVariables|SetRand (Math|Random|RandomFloatinRange 0.0 3.6e+02)))
  (if (CallFunction|CanSpawnArea (+ _returnvalue_2 (Math|Vector|MakeVector (* (Math|Trig|Cos(Radians) _output_get) _returnvalue_3) (* (Math|Trig|Sin(Radians) _output_get) _returnvalue_3) 0.0) "0.000000,0.000000,5.000000"))
    (bind _outrownames (DataTable|GetDataTableRowNames "/Game/00/Monster/DT_monster.DT_monster"))
    (bind _returnvalue_4 (Utilities|GetDataTableRow "/Game/00/Monster/DT_monster.DT_monster" (.OutItem (Utilities|Array|Random _outrownames)))
      (:then
        (bind _returnvalue_5 (AI|SpawnAIFromClass (.MonsterClass (Utilities|Struct|BreakST_Moster _returnvalue_4)) "/Game/00/Monster/BT_Monster.BT_Monster" (+ _returnvalue_2 (Math|Vector|MakeVector (* (Math|Trig|Cos(Radians) _output_get) _returnvalue_3) (* (Math|Trig|Sin(Radians) _output_get) _returnvalue_3) 0.0) "0.000000,0.000000,5.000000") (Math|Rotator|FindLookatRotation (+ _returnvalue_2 (Math|Vector|MakeVector (* (Math|Trig|Cos(Radians) _output_get) _returnvalue_3) (* (Math|Trig|Sin(Radians) _output_get) _returnvalue_3) 0.0) "0.000000,0.000000,5.000000") _returnvalue_2) false 0))
        (bind _asbp_monster_base (Utilities|Casting|CastToBP_Monster_Base _returnvalue_5))
        (Default|InitMonsterInfo _asbp_monster_base _returnvalue_4)))))

(fn CanSpawnArea
  (params (Loction :type Vector))
  (bind _returnvalue (Collision|LineTraceForObjects Loction (* Loction "0.000000,0.000000,-100.000000") (Utilities|Array|MakeArray "ObjectTypeQuery2") false 0 "None"))
  (return _returnvalue))