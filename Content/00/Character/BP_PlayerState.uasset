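; BP_PlayerState holds a character's current and max HP and handles healing, damage and death checks.
; On BeginPlay it fills HP to max, and every HP change fires the UpdateHP dispatcher with current and max values.
; AddDamage ignores hits once dead and otherwise returns whether the hit was fatal.
; Heal and damage apply without clamping, and healing has no death check.
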(event EventBeginPlay
  (CallFunction|SetCurHp (Variables|Default|GetMaxHp)))

(fn ConstructionScript)

(fn AddHeal
  (params (Heal :type Float%20%28double-precision%29))
  (bind _output_get (Variables|Default|SetCurHp (+ (Variables|Default|GetCurHp) Heal)))
  (Default|CallEventDispatcherUpdateHP _output_get (Variables|Default|GetMaxHp)))

(fn AddDamage
  (params (Damage :type Float%20%28double-precision%29))
  (if (CallFunction|IsDeath)
    (return false)
    (else
      (Utilities|FlowControl|Sequence
        (:then_0
          (bind _output_get (Variables|Default|SetCurHp (- (Variables|Default|GetCurHp) Damage)))
          (Default|CallEventDispatcherUpdateHP _output_get (Variables|Default|GetMaxHp)))
        (:then_1
          (return (CallFunction|IsDeath)))))))

(fn SetCurHp
  (params (CurHp :type Float%20%28double-precision%29))
  (bind _output_get (Variables|Default|SetCurHp CurHp))
  (Default|CallEventDispatcherUpdateHP _output_get (Variables|Default|GetMaxHp)))

(fn IsDeath
  (return (<= (Variables|Default|GetCurHp) 0.0)))