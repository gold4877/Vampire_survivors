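; Player character with Enhanced Input movement and running, three named skills and an HP name tag.
; BeginPlay binds the name tag to the PlayerState's HP dispatcher and adds Slash, Projectile and ShieldAura to the skill component.
; Damage goes to the PlayerState; a true result changes the game state, pauses and switches to UI-only input.
; Look input is unwired, leaving its yaw and pitch nodes unused.
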(event Input|EnhancedActionEvents|EnhancedInputActionIA_Look
  (params (ActionValue :type Vector%202D%20Structure) (ElapsedSeconds :type Float%20%28double-precision%29) (TriggeredSeconds :type Float%20%28double-precision%29) (InputAction :type Input%20Action%20Object%20Reference :default "/Game/ThirdPerson/Input/Actions/IA_Look.IA_Look")))

(event Input|EnhancedActionEvents|EnhancedInputActionIA_Move
  (params (ActionValue :type Vector%202D%20Structure) (ElapsedSeconds :type Float%20%28double-precision%29) (TriggeredSeconds :type Float%20%28double-precision%29) (InputAction :type Input%20Action%20Object%20Reference :default "/Game/ThirdPerson/Input/Actions/IA_Move.IA_Move"))
  (bind _returnvalue (Pawn|GetControlRotation :!class /Script/Engine.Pawn))
  (Pawn|Input|AddMovementInput (Math|Vector|GetRightVector (Math|Rotator|MakeRotator (.roll _returnvalue) 0.0 (.yaw _returnvalue))) (.x ActionValue) false)
  (Pawn|Input|AddMovementInput (Math|Vector|GetForwardVector (Math|Rotator|MakeRotator 0.0 0.0 (.yaw _returnvalue))) (.y ActionValue) false))

(event Input|EnhancedActionEvents|EnhancedInputActionIA_Run
  (params (ActionValue :type Boolean) (ElapsedSeconds :type Float%20%28double-precision%29) (TriggeredSeconds :type Float%20%28double-precision%29) (InputAction :type Input%20Action%20Object%20Reference :default "/Game/00/IA_Run.IA_Run"))
  (bind _charactermovement (Variables|Character|GetCharacterMovement))
  (:Started
    (Variables|/Script/Engine.CharacterMovementComponent|SetMaxWalkSpeed _charactermovement 6e+02))
  (:Completed
    (Variables|/Script/Engine.CharacterMovementComponent|SetMaxWalkSpeed _charactermovement 4e+02)))

(event EventBeginPlay
  (Utilities|FlowControl|Sequence
    (:then_0
      (CallFunction|InitChar))
    (:then_1
      (Default|AddSkill (Variables|Default|GetBP_SkillComponent) "Slash")
      (Default|AddSkill (Variables|Default|GetBP_SkillComponent) "Projectile")
      (Default|AddSkill (Variables|Default|GetBP_SkillComponent) "ShieldAura"))))

(event Game|Damage|EventAnyDamage
  (params (Damage :type Float%20%28single-precision%29) (DamageType :type Damage%20Type%20Object%20Reference) (InstigatedBy :type Controller%20Object%20Reference) (DamageCauser :type Actor%20Object%20Reference))
  (bind _returnvalue (Game|GetPlayerController 0))
  (bind _asbp_player_state (Utilities|Casting|CastToBP_PlayerState (Variables|GetPlayerState)))
  (bind _isjustdeath (Default|AddDamage _asbp_player_state Damage))
  (if _isjustdeath
    (bind _asbp_game_state (Utilities|Casting|CastToBP_gameState (Game|GetGameState)))
    (Default|ChangeGmaeState _asbp_game_state "NewEnumerator3")
    (Game|SetGamePaused true)
    (Input|SetInputModeUIOnly _returnvalue 0 "DoNotLock" false)
    (Variables|/Script/Engine.PlayerController|SetbShowMouseCursor _returnvalue true)))

(event EventControllerChanged
  (params (OldController :type Controller%20Object%20Reference) (NewController :type Controller%20Object%20Reference))
  (bind _asplayer_controller (Utilities|Casting|CastToPlayerController NewController))
  (Input|AddMappingContext (PlayerController|LocalPlayerSubsystems|GetEnhancedInputLocalPlayerSubsystem _asplayer_controller) "/Game/00/IMC_Character.IMC_Character" 0 "(bIgnoreAllPressedKeysUntilRelease=True,bForceImmediately=False,bNotifyUserSettings=False)"))

(fn ConstructionScript)

(fn InitChar
  (bind _asbp_player_state (Utilities|Casting|CastToBP_PlayerState (Variables|GetPlayerState)))
  (EventDispatchers|BindEventtoEventDispatcherUpdateHP _asbp_player_state (EventDispatchers|CreateEvent :!event EventUpdateHp))
  (Default|UpdateHp (Variables|Default|GetNameTagComponent) (Variables|/Game/00/Character/BP_PlayerState.BP_PlayerState_C|GetCurHp _asbp_player_state) (Variables|/Game/00/Character/BP_PlayerState.BP_PlayerState_C|GetMaxHp _asbp_player_state)))

(fn EventUpdateHp
  (params (CurHp :type Float%20%28double-precision%29) (MaxHp :type Float%20%28double-precision%29))
  (Default|UpdateHp (Variables|Default|GetNameTagComponent) CurHp MaxHp))