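; Projectile skill actor that flies forward and deals damage over time to the monsters it passes through.
; Tick moves it along its forward vector at Speed without sweeping, and a timer destroys it after a fixed lifetime.
; A looping timer damages every BP_Monster_Base overlapping its hit collision, scaling SkillInfo damage by the timer interval and crediting the first player controller.
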(event EventTick
  (params (DeltaSeconds :type Float%20%28single-precision%29))
  (Transformation|AddActorWorldOffset (* (* DeltaSeconds (Variables|Default|GetSpeed)) (Transformation|GetActorForwardVector))))

(event EventBeginPlay
  (Utilities|Time|SetTimerbyFunctionName 0 "DoDestroy" 3.0)
  (Utilities|Time|SetTimerbyFunctionName 0 "DoDamage" (Variables|Default|GetTimerDS) true true))

(fn ConstructionScript)

(fn DoDestroy
  (Actor|DestroyActor))

(fn DoDamage
  (for _array_element (Collision|GetOverlappingActors (Variables|Default|GetHitCollsion) "/Game/00/Monster/BP_Monster_Base.BP_Monster_Base_C" :!class /Script/Engine.PrimitiveComponent)
    (Game|Damage|ApplyDamage _array_element (* (.damage (Variables|Default|GetSkillInfo)) (Variables|Default|GetTimerDS)) (Game|GetPlayerController 0) self)))