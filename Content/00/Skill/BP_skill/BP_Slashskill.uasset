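; BP_Slashskill is a slash skill actor that deals a one-time burst of area damage to monsters.
; On BeginPlay it attaches to its Instigator, keeping its world transform, and applies SkillInfo damage to every BP_Monster_Base overlapping its Sphere, credited to player controller 0.
; It also binds to the finish events of its lightning slash and attack effect systems, with EventEffectFinish destroying the actor.
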(event EventBeginPlay
  (Transformation|AttachActorToActor (Game|GetInstigator) "None" "KeepWorld" "KeepWorld" "KeepWorld" true)
  (EventDispatchers|BindEventtoOnSystemFinished (Variables|Default|GetNS_LightningSlash) (EventDispatchers|CreateEvent :!event EventEffectFinish))
  (CallFunction|DoDamage))

(fn ConstructionScript)

(fn EventEffectFinish
  (params (PSystem :type Niagara%20Component%20Object%20Reference))
  (Actor|DestroyActor))

(fn DoDamage
  (for _array_element (Collision|GetOverlappingActors (Variables|Default|GetSphere) "/Game/00/Monster/BP_Monster_Base.BP_Monster_Base_C" :!class /Script/Engine.PrimitiveComponent)
    (Game|Damage|ApplyDamage _array_element (.damage (Variables|Default|GetSkillInfo)) (Game|GetPlayerController 0) self)))