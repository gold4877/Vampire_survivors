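; BP_ShiedAura is a short-lived skill actor: a rotating aura that follows its instigator and damages monsters it overlaps.
; Tick spins it around yaw and snaps it to the instigator's location.
; A looping timer damages every BP_Monster_Base inside HitCollsion, scaling SkillInfo.Damage by the interval so it acts as damage per second, credited to player controller 0.
; A second timer destroys the actor after a fixed lifetime.
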(event EventTick
  (params (DeltaSeconds :type Float%20%28single-precision%29))
  (Utilities|FlowControl|Sequence
    (:then_0
      (Class|Actor|AddActorWorldRotation (Math|Rotator|MakeRotator 0.0 0.0 (* DeltaSeconds (Variables|Default|GetSpeed)))))
    (:then_1
      (Transformation|SetActorLocation (Transformation|GetActorLocation (Game|GetInstigator)) false false))))

(event EventBeginPlay
  (Utilities|Time|SetTimerbyFunctionName 0 "DoDestorySkill" 5.0)
  (Utilities|Time|SetTimerbyFunctionName 0 "DoDamage" (Variables|Default|GetTimerDS) true true))

(fn ConstructionScript)

(fn DoDestorySkill
  (Actor|DestroyActor))

(fn DoDamage
  (for _array_element (Collision|GetOverlappingActors (Variables|Default|GetHitCollsion) "/Game/00/Monster/BP_Monster_Base.BP_Monster_Base_C" :!class /Script/Engine.PrimitiveComponent)
    (Game|Damage|ApplyDamage _array_element (* (.damage (Variables|Default|GetSkillInfo)) (Variables|Default|GetTimerDS)) (Game|GetPlayerController 0) self)))