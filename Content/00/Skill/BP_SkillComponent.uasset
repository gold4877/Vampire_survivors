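; BP_SkillComponent is an actor component that automatically fires its owner's skills on repeating timers.
; AddSkill looks up a row in DT_skill and stores it with a countdown starting at that skill's SpawnDelay.
; Tick decrements each countdown; below zero, it adds the delay back, preserving overshoot, and calls DoFireSkill.
; DoFireSkill spawns the skill's BP_SkillBase class at the owner's transform, passing the skill info and owning Pawn as Instigator.
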(event EventBeginPlay)

(event EventTick
  (params (DeltaSeconds :type Float%20%28single-precision%29))
  (CallFunction|UpdateSkills DeltaSeconds))

(fn DoFireSkill
  (params (Skill :type ST%20Skill%20Structure))
  (bind _returnvalue (Components|GetOwner))
  (bind _aspawn (Utilities|Casting|CastToPawn _returnvalue))
  (bind _asbp_skill_base (Utilities|Casting|CastToBP_SkillBaseClass (.SpawnActor (Utilities|Struct|BreakST_skill Skill))))
  (Game|SpawnActorfromClass _asbp_skill_base (Transformation|GetActorTransform _returnvalue) "Undefined" "MultiplyWithRoot" 0 Skill _aspawn))

(fn AddSkill
  (params (SkillName :type Name))
  (bind _returnvalue (Utilities|GetDataTableRow "/Game/00/Skill/DT_skill.DT_skill" SkillName)
    (:then
      (Utilities|Array|Add (Variables|Default|GetSkills) (Utilities|Struct|MakeST_SkillRef _returnvalue (.SpawnDelay (Utilities|Struct|BreakST_skill _returnvalue)))))))

(fn UpdateSkills
  (params (DeltaSeconds :type Float%20%28double-precision%29))
  (bind _skills (Variables|Default|GetSkills))
  (for (_ _array_index) _skills
    (CallFunction|UpdateSkillRef (Utilities|Array|Get(acopy) _skills _array_index) DeltaSeconds)))

(fn UpdateSkillRef
  (params (SkillRef :type ST%20Skill%20Ref%20Structure%20%28by%20ref%29) (DeltaSeconds :type Float%20%28double-precision%29))
  (bind (_skill _curtime) (Utilities|Struct|BreakST_SkillRef SkillRef))
  (bind _structout (Utilities|Struct|SetmembersinST_SkillRef SkillRef (- (.CurTime (Utilities|Struct|BreakST_SkillRef SkillRef)) DeltaSeconds)))
  (if (< (.CurTime (Utilities|Struct|BreakST_SkillRef _structout)) 0.0)
    (Utilities|Struct|SetmembersinST_SkillRef SkillRef (+ _curtime (.SpawnDelay (Utilities|Struct|BreakST_skill (.Skill (Utilities|Struct|BreakST_SkillRef _structout))))))
    (CallFunction|DoFireSkill _skill)))